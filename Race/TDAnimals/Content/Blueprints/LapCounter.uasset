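; LapCounter is a Blueprint that detects lap completion for RunningAnimalBase actors using three trigger boxes.
; Each box overlap writes the animal's LapState, giving StartBox, MidBox and EndBox their own state.
; StartBox reports a new lap only if the state is still EndBox's, so a later MidBox overlap invalidates it.
; Laps are only printed as debug strings, with no count stored.
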(event OnComponentBeginOverlap(StartBox)
  (params (OverlappedComponent :type Primitive%20Component%20Object%20Reference) (OtherActor :type Actor%20Object%20Reference) (OtherComp :type Primitive%20Component%20Object%20Reference) (OtherBodyIndex :type Integer) (bFromSweep :type Boolean) (SweepResult :type Hit%20Result%20Structure%20%28by%20ref%29))
  (bind _asrunning_animal_base (Utilities|Casting|CastToRunningAnimalBase OtherActor))
  (Utilities|FlowControl|Sequence
    (:then_0
      (if (Utilities|Enum|Equal(Enum) (Variables|/Game/Characters/RunningAnimalBase.RunningAnimalBase_C|GetLapState _asrunning_animal_base) "NewEnumerator2")
        (Development|PrintString "New lap!")))
    (:then_1
      (Variables|/Game/Characters/RunningAnimalBase.RunningAnimalBase_C|SetLapState _asrunning_animal_base "NewEnumerator0")
      (Development|PrintString "Start"))))

(event OnComponentBeginOverlap(EndBox)
  (params (OverlappedComponent :type Primitive%20Component%20Object%20Reference) (OtherActor :type Actor%20Object%20Reference) (OtherComp :type Primitive%20Component%20Object%20Reference) (OtherBodyIndex :type Integer) (bFromSweep :type Boolean) (SweepResult :type Hit%20Result%20Structure%20%28by%20ref%29))
  (bind _asrunning_animal_base (Utilities|Casting|CastToRunningAnimalBase OtherActor))
  (Variables|/Game/Characters/RunningAnimalBase.RunningAnimalBase_C|SetLapState _asrunning_animal_base "NewEnumerator2")
  (Development|PrintString "end"))

(event OnComponentBeginOverlap(MidBox)
  (params (OverlappedComponent :type Primitive%20Component%20Object%20Reference) (OtherActor :type Actor%20Object%20Reference) (OtherComp :type Primitive%20Component%20Object%20Reference) (OtherBodyIndex :type Integer) (bFromSweep :type Boolean) (SweepResult :type Hit%20Result%20Structure%20%28by%20ref%29))
  (bind _asrunning_animal_base (Utilities|Casting|CastToRunningAnimalBase OtherActor))
  (Variables|/Game/Characters/RunningAnimalBase.RunningAnimalBase_C|SetLapState _asrunning_animal_base "NewEnumerator1")
  (Development|PrintString "INvalidate"))

(event EventBeginPlay)

(event EventTick
  (params (DeltaSeconds :type Float%20%28single-precision%29)))

(event Collision|EventActorBeginOverlap
  (params (OtherActor :type Actor%20Object%20Reference)))

(fn ConstructionScript)