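; Race manager that runs an animal race from countdown to results screen, with restart and return-to-select handlers.
; On BeginPlay it possesses pre-placed RunningAnimalBase pawns from GameInstance player data, fills up to four racers with unchosen animal types as AI, and destroys the rest.
; A looping timer drives the HUD countdown and unlocks movement; Tick accumulates race times until all finish.
; A Disable flag bypasses race setup, letting tagged animals run as AI.
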(event EventBeginPlay
  (bind _self self)
  (bind _instance (CallFunction|GetAnimalGameInstance _self))
  ;[1 1 1] Spawn racers / Start race countdown
  ;[1 1 1] Deactivate
  (if (Variables|Default|GetDisable)
    (bind _outactors (Actor|GetAllActorsOfClasswithTag "/Game/Characters/RunningAnimalBase.RunningAnimalBase_C" "ManagerHorse"))
    (for _array_element _outactors
      (Actor|DestroyActor _array_element))
    (Input|AddMappingContext (PlayerController|LocalPlayerSubsystems|GetEnhancedInputLocalPlayerSubsystem (Game|GetPlayerController 0)) "/Game/Input/IMC_Default.IMC_Default" 0 "(bIgnoreAllPressedKeysUntilRelease=True,bForceImmediately=False,bNotifyUserSettings=False)")
    (bind _outactors_2 (Actor|GetAllActorsOfClass "/Game/Characters/RunningAnimalBase.RunningAnimalBase_C"))
    (for _array_element_2 _outactors_2
      (Variables|/Game/Characters/RunningAnimalBase.RunningAnimalBase_C|SetMovementAllowed%20 _array_element_2 true)
      (Variables|/Game/Characters/RunningAnimalBase.RunningAnimalBase_C|SetIsAI _array_element_2 true))
    (else
      (bind _outactors_3 (Actor|GetAllActorsOfClasswithTag "/Game/Characters/RunningAnimalBase.RunningAnimalBase_C" "NoManagerHorse"))
      (for _array_element_3 _outactors_3
        (Actor|DestroyActor _array_element_3))
      (Variables|Default|SetCurrentRacePlayerData (Variables|/Game/Blueprints/BP_Game_Instance.BP_Game_Instance_C|GetPlayerData _instance))
      (Variables|Default|SetCurrentRaceCharacterRoster (Variables|/Game/Blueprints/BP_Game_Instance.BP_Game_Instance_C|GetCharacterRoster _instance))
      (bind _returnvalue (UserInterface|CreateWidget "/Game/Blueprints/RaceLogic/WB_RaceUI.WB_RaceUI_C"))
      (bind _output_get (Variables|Default|SetRaceHUDRef _returnvalue))
      (UserInterface|Viewport|AddtoViewport _output_get 0)
      (CallFunction|SpawnPlayers)
      (CallFunction|StartRaceCountdown))))

(event EventTick
  (params (DeltaSeconds :type Float%20%28single-precision%29))
  ;[1 1 1] Track player time
  (if (Variables|Default|GetRaceInProgress)
    (for _array_element (Variables|Default|GetActiveRacePawns)
      (if (not (Variables|/Game/Characters/RunningAnimalBase.RunningAnimalBase_C|GetFinishedRace _array_element))
        (Variables|/Game/Characters/RunningAnimalBase.RunningAnimalBase_C|SetRaceTime _array_element (+ DeltaSeconds (Variables|/Game/Characters/RunningAnimalBase.RunningAnimalBase_C|GetRaceTime _array_element)))))
    ;[1 1 1] Check if all players finished, show results if they have
    (bind _racefinished (CallFunction|CheckifAllPlayersFinished))
    (if _racefinished
      (Default|ShowResultsScreen (Variables|Default|GetRaceHUDRef) (Variables|Default|GetActiveRacePawns)))))

(event Collision|EventActorBeginOverlap
  (params (OtherActor :type Actor%20Object%20Reference)))

(fn ConstructionScript)

(fn SpawnPlayers
  ;[1 1 1] Setup/clearing lists
  (bind _outactors (Actor|GetAllActorsOfClass "/Game/Characters/RunningAnimalBase.RunningAnimalBase_C"))
  (LocalVariables|SetPrePlacedPawns _outactors)
  (Utilities|Array|Clear (Variables|Default|GetActiveRacePawns))
  (Utilities|Array|Clear (LocalVariables|GetSelectedAnimalTypes))
  ;[1 1 1] Loop player slots
  (for _array_element (Variables|/Game/Blueprints/BP_Game_Instance.BP_Game_Instance_C|GetPlayerData (CallFunction|GetAnimalGameInstance self))
    ;;[1 1 1] Is AI check
    (if (not (.bIsAI (Utilities|Struct|BreakS_PlayerData _array_element)))
      (Utilities|Array|AddUnique (LocalVariables|GetSelectedAnimalTypes) (.ChosenCharacter (Utilities|Struct|BreakS_PlayerData _array_element)))
      ;[1 1 1] Find human pawn
      (bind _array_element_2 (Utilities|Array|ForEachLoopwithBreak (LocalVariables|GetPrePlacedPawns))
        (:LoopBody
          ;;[1 1 1] Correct animal type check
          (if (Utilities|Enum|Equal(Enum) (Variables|/Game/Characters/RunningAnimalBase.RunningAnimalBase_C|GetAnimalType _array_element_2) (.ChosenCharacter (Utilities|Struct|BreakS_PlayerData _array_element)))
            ;;[1 1 1] Is pawn available check
            (if (not (Utilities|Array|ContainsItem (Variables|Default|GetActiveRacePawns) _array_element_2))
              (Variables|/Game/Characters/RunningAnimalBase.RunningAnimalBase_C|SetIsAI _array_element_2 false)
              ;;[1 1 1] Valid controller check
              (if (!= (.ControllerID (Utilities|Struct|BreakS_PlayerData _array_element)) -1)
                (Utilities|Array|Add (Variables|Default|GetActiveRacePawns) _array_element_2)
                (Pawn|Possess (Game|GetPlayerController (.ControllerID (Utilities|Struct|BreakS_PlayerData _array_element))) _array_element_2))))))))
  ;[1 1 1] Select AI
  (bind _array_element_3 (Utilities|Array|ForEachLoopwithBreak (LocalVariables|GetPrePlacedPawns) :!label _label)
    (:LoopBody
      ;;[1 1 1] Is race full check
      (if (>= (Utilities|Array|Length (Variables|Default|GetActiveRacePawns)) 4)
        (goto _label Break)
        (else
          ;;[1 1 1] Pawn already human check
          (if (not (Utilities|Array|ContainsItem (Variables|Default|GetActiveRacePawns) _array_element_3))
            ;;[1 1 1] Animal type taken check
            (if (not (Utilities|Array|ContainsItem (LocalVariables|GetSelectedAnimalTypes) (Variables|/Game/Characters/RunningAnimalBase.RunningAnimalBase_C|GetAnimalType _array_element_3)))
              (Variables|/Game/Characters/RunningAnimalBase.RunningAnimalBase_C|SetIsAI _array_element_3 true)
              (Utilities|Array|Add (Variables|Default|GetActiveRacePawns) _array_element_3)
              (Utilities|Array|AddUnique (LocalVariables|GetSelectedAnimalTypes) (Variables|/Game/Characters/RunningAnimalBase.RunningAnimalBase_C|GetAnimalType _array_element_3)))))))
    (:Completed
      ;[1 1 1] Delete unused pawns
      (for _array_element_4 (LocalVariables|GetPrePlacedPawns)
        (if (not (Utilities|Array|ContainsItem (Variables|Default|GetActiveRacePawns) _array_element_4))
          (Actor|DestroyActor _array_element_4)))
      (return))))

(fn StartRaceCountdown
  (Variables|Default|SetRaceInProgress false)
  (Variables|Default|SetCurrentCountdownValue (Variables|Default|GetRaceCountdownDuration))
  ;[1 1 1] Disable movement
  (for _array_element (Variables|Default|GetActiveRacePawns)
    (Variables|/Game/Characters/RunningAnimalBase.RunningAnimalBase_C|SetMovementAllowed%20 _array_element false))
  (Default|UpdateCountdownDisplay (Variables|Default|GetRaceHUDRef) (Variables|Default|GetCurrentCountdownValue))
  (bind _returnvalue (Utilities|Time|SetTimerbyFunctionName 0 "TickRaceCountdown" 1.0 true))
  (Variables|Default|SetCountdownTimerHandle _returnvalue))

(fn TickRaceCountdown
  (bind _output_get (Variables|Default|SetCurrentCountdownValue (- (Variables|Default|GetCurrentCountdownValue) 1)))
  (Default|UpdateCountdownDisplay (Variables|Default|GetRaceHUDRef) _output_get)
  (if (<= (Variables|Default|GetCurrentCountdownValue) 0)
    (Utilities|Time|ClearandInvalidateTimerbyHandle (Variables|Default|GetCountdownTimerHandle))
    (Variables|Default|SetRaceInProgress true)
    (Default|HideCountdownDisplay (Variables|Default|GetRaceHUDRef))
    (for _array_element (Variables|Default|GetActiveRacePawns)
      (Variables|/Game/Characters/RunningAnimalBase.RunningAnimalBase_C|SetMovementAllowed%20 _array_element true))))

(fn CheckifAllPlayersFinished
  (bind _array_element (Utilities|Array|ForEachLoopwithBreak (Variables|Default|GetActiveRacePawns) :!label _label)
    (:LoopBody
      (if (not (Variables|/Game/Characters/RunningAnimalBase.RunningAnimalBase_C|GetFinishedRace _array_element))
        (LocalVariables|SetSomeoneStillRacing true)
        (goto _label Break)))
    (:Completed
      (if (not (LocalVariables|GetSomeoneStillRacing))
        (bind _output_get (Variables|/Game/Characters/RunningAnimalBase.RunningAnimalBase_C|SetFinishedRace _array_element true))
        (Variables|Default|SetRaceInProgress false)
        (return _output_get)))))

(fn SwitchtoResultsInput
  (for _index (range 0 3)
    (Utilities|IsValid (Game|GetPlayerController _index)
      (:Is%20Valid
        (Input|RemoveMappingContext (PlayerController|LocalPlayerSubsystems|GetEnhancedInputLocalPlayerSubsystem (Game|GetPlayerController _index)) "/Game/Input/IMC_Default.IMC_Default" "(bIgnoreAllPressedKeysUntilRelease=True,bForceImmediately=False,bNotifyUserSettings=False)")
        (Input|AddMappingContext (PlayerController|LocalPlayerSubsystems|GetEnhancedInputLocalPlayerSubsystem (Game|GetPlayerController _index)) "/Game/Input/IMC_ResultsScreen.IMC_ResultsScreen" 0 "(bIgnoreAllPressedKeysUntilRelease=True,bForceImmediately=False,bNotifyUserSettings=False)")))))

(fn HandleRestartRace
  (bind _returnvalue (Game|GetCurrentLevelName true))
  (Game|OpenLevel(byName) (Utilities|String|StringToName _returnvalue)))

(fn HandleReturntoSelect
  (Game|OpenLevel(byName) "L_CharSelect"))