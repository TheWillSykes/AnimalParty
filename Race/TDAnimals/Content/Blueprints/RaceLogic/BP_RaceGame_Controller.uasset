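; BP_RaceGame_Controller is the race game controller that routes restart-race and return-to-select input to the RaceGameManager.
; On BeginPlay it finds and caches the manager, then adds the default Enhanced Input mapping context for each valid player controller among the first four indices, covering local multiplayer.
; The two input action events only forward to the manager's handler functions, so the race logic itself lives there.
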(event Input|EnhancedActionEvents|EnhancedInputActionIA_RestartRace
  (params (ActionValue :type Boolean) (ElapsedSeconds :type Float%20%28double-precision%29) (TriggeredSeconds :type Float%20%28double-precision%29) (InputAction :type Input%20Action%20Object%20Reference :default "/Game/Input/Actions/IA_RestartRace.IA_RestartRace"))
  ;[1 1 1] Restart race
  (:Started
    (Default|HandleRestartRace (Variables|Default|GetGameManager))))

(event Input|EnhancedActionEvents|EnhancedInputActionIA_ReturnToSelect
  (params (ActionValue :type Boolean) (ElapsedSeconds :type Float%20%28double-precision%29) (TriggeredSeconds :type Float%20%28double-precision%29) (InputAction :type Input%20Action%20Object%20Reference :default "/Game/Input/Actions/IA_ReturnToSelect.IA_ReturnToSelect"))
  ;[1 1 1] Return to select
  (:Started
    (Default|HandleReturntoSelect (Variables|Default|GetGameManager))))

(event EventBeginPlay
  (bind _outactors (Actor|GetAllActorsOfClass "/Game/Blueprints/RaceLogic/RaceGameManager.RaceGameManager_C"))
  (for _array_element _outactors
    ;[1 1 1] Race mapping
    (Variables|Default|SetGameManager _array_element)
    (for _index (range 0 3)
      (Utilities|IsValid (Game|GetPlayerController _index)
        (:Is%20Valid
          (Input|AddMappingContext (PlayerController|LocalPlayerSubsystems|GetEnhancedInputLocalPlayerSubsystem (Game|GetPlayerController _index)) "/Game/Input/IMC_Default.IMC_Default" 0 "(bIgnoreAllPressedKeysUntilRelease=True,bForceImmediately=False,bNotifyUserSettings=False)"))))))

(fn ConstructionScript)