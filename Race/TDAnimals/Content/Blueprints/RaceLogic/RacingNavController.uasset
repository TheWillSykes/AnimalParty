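; Racing navigation actor that holds an ordered array of nodes forming a closed loop for the race logic.
; The construction script starts a looping timer on DebugDraw, which draws arrows between consecutive nodes and from last back to first.
; DebugDraw also writes each node's ID from its array index, so numbering depends on that debug pass.
; GetNextNavNodeID returns the following index, wrapping at the end of the array.
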(event EventBeginPlay)

(event Collision|EventActorBeginOverlap
  (params (OtherActor :type Actor%20Object%20Reference)))

(event EventTick
  (params (DeltaSeconds :type Float%20%28single-precision%29)))

(fn ConstructionScript
  (Utilities|Time|SetTimerbyFunctionName 0 "DebugDraw" 0.1 true true))

(fn DebugDraw
  (bind _nodes (Variables|Default|GetNodes))
  (LocalVariables|SetPrev 0)
  (for (_array_element _array_index) (Variables|Default|GetNodes)
    (Variables|/Game/Blueprints/RaceLogic/RacingNavNode.RacingNavNode_C|SetID _array_element _array_index)
    (Utilities|FlowControl|Sequence
      (:then_0
        (Utilities|IsValid (LocalVariables|GetPrev)
          (:Is%20Valid
            (Rendering|Debug|DrawDebugArrow :LineStart (+ (Transformation|GetActorLocation (LocalVariables|GetPrev)) "0.000000,0.000000,10.000000") :LineEnd (+ (Transformation|GetActorLocation _array_element) "0.000000,0.000000,10.000000") :Duration 0.1 :Thickness 1e+01))))
      (:then_1
        (LocalVariables|SetPrev _array_element))))
  (Rendering|Debug|DrawDebugArrow :LineStart (+ (Transformation|GetActorLocation (Utilities|Array|Get(acopy) _nodes (Utilities|Array|LastIndex _nodes))) "0.000000,0.000000,10.000000") :LineEnd (+ (Transformation|GetActorLocation (Utilities|Array|Get(acopy) _nodes)) "0.000000,0.000000,10.000000") :Duration 0.1 :Thickness 1e+01))

(fn GetNextNavNodeID
  (params (NodeID :type Integer))
  (return (Math|Integer|%(Integer) (+ NodeID 1) (Utilities|Array|Length (Variables|Default|GetNodes)))))