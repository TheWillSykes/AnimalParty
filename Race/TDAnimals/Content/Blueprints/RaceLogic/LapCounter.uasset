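; Lap counter actor that tracks laps and race completion for RunningAnimalBase racers.
; Start, Mid and End trigger boxes each stamp the overlapping racer's LapState, without Mid or End checking the previous state.
; Start first increments CurrentLap if the racer last hit End, then sets FinishedRace once it reaches TotalLapsToWin from the RaceGameManager found at BeginPlay.
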(event OnComponentBeginOverlap(StartBox)
  (params (OverlappedComponent :type Primitive%20Component%20Object%20Reference) (OtherActor :type Actor%20Object%20Reference) (OtherComp :type Primitive%20Component%20Object%20Reference) (OtherBodyIndex :type Integer) (bFromSweep :type Boolean) (SweepResult :type Hit%20Result%20Structure%20%28by%20ref%29))
  (bind _asrunning_animal_base (Utilities|Casting|CastToRunningAnimalBase OtherActor))
  (Utilities|FlowControl|Sequence
    (:then_0
      (if (Utilities|Enum|Equal(Enum) (Variables|/Game/Characters/RunningAnimalBase.RunningAnimalBase_C|GetLapState _asrunning_animal_base) "NewEnumerator2")
        ;[1 1 1] Sets new lap to current lap
        (Variables|/Game/Characters/RunningAnimalBase.RunningAnimalBase_C|SetCurrentLap _asrunning_animal_base (+ (Variables|/Game/Characters/RunningAnimalBase.RunningAnimalBase_C|GetCurrentLap _asrunning_animal_base) 1))
        ;[1 1 1] Finishes the race if all laps are finished
        (if (>= (Variables|/Game/Characters/RunningAnimalBase.RunningAnimalBase_C|GetCurrentLap _asrunning_animal_base) (Variables|/Game/Blueprints/RaceLogic/RaceGameManager.RaceGameManager_C|GetTotalLapsToWin (Variables|Default|GetGame%20Manager)))
          (Variables|/Game/Characters/RunningAnimalBase.RunningAnimalBase_C|SetFinishedRace _asrunning_animal_base true))))
    (:then_1
      (Variables|/Game/Characters/RunningAnimalBase.RunningAnimalBase_C|SetLapState _asrunning_animal_base "NewEnumerator0"))))

(event OnComponentBeginOverlap(EndBox)
  (params (OverlappedComponent :type Primitive%20Component%20Object%20Reference) (OtherActor :type Actor%20Object%20Reference) (OtherComp :type Primitive%20Component%20Object%20Reference) (OtherBodyIndex :type Integer) (bFromSweep :type Boolean) (SweepResult :type Hit%20Result%20Structure%20%28by%20ref%29))
  (bind _asrunning_animal_base (Utilities|Casting|CastToRunningAnimalBase OtherActor))
  (Variables|/Game/Characters/RunningAnimalBase.RunningAnimalBase_C|SetLapState _asrunning_animal_base "NewEnumerator2"))

(event OnComponentBeginOverlap(MidBox)
  (params (OverlappedComponent :type Primitive%20Component%20Object%20Reference) (OtherActor :type Actor%20Object%20Reference) (OtherComp :type Primitive%20Component%20Object%20Reference) (OtherBodyIndex :type Integer) (bFromSweep :type Boolean) (SweepResult :type Hit%20Result%20Structure%20%28by%20ref%29))
  (bind _asrunning_animal_base (Utilities|Casting|CastToRunningAnimalBase OtherActor))
  (Variables|/Game/Characters/RunningAnimalBase.RunningAnimalBase_C|SetLapState _asrunning_animal_base "NewEnumerator1"))

(event EventBeginPlay
  (bind _outactors (Actor|GetAllActorsOfClass "/Game/Blueprints/RaceLogic/RaceGameManager.RaceGameManager_C"))
  (for _array_element _outactors
    (Variables|Default|SetGame%20Manager _array_element)))

(event EventTick
  (params (DeltaSeconds :type Float%20%28single-precision%29)))

(fn ConstructionScript)