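; Character select player controller that lets each local player join, cycle characters and continue to the next screen.
; On begin play it finds the CharSelectGameManager and, after a short delay, adds the character select Enhanced Input context with Game and UI input mode.
; Join, horizontal navigation and continue inputs forward to the manager, keyed by the stored player index.
; Continue also adds the default mapping context for gameplay.
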(event Input|EnhancedActionEvents|EnhancedInputActionIA_Join
  (params (ActionValue :type Boolean) (ElapsedSeconds :type Float%20%28double-precision%29) (TriggeredSeconds :type Float%20%28double-precision%29) (InputAction :type Input%20Action%20Object%20Reference :default "/Game/Input/Actions/IA_Join.IA_Join"))
  (bind _game_manager (Variables|Default|GetGame%20Manager))
  (bind _myplayerindex (Variables|Default|GetMyPlayerIndex))
  ;[1 1 1] Input trigger for player joining the game
  (:Started
    (if (== _myplayerindex -1)
      (Default|HandlePlayerJoinAttempt _game_manager self)
      (Default|HandleCharacterSelection _game_manager _myplayerindex 0.0))))

(event Input|EnhancedActionEvents|EnhancedInputActionIA_ActivateContinue
  (params (ActionValue :type Boolean) (ElapsedSeconds :type Float%20%28double-precision%29) (TriggeredSeconds :type Float%20%28double-precision%29) (InputAction :type Input%20Action%20Object%20Reference :default "/Game/Input/Actions/IA_ActivateContinue.IA_ActivateContinue"))
  ;[1 1 1] Input trigger for player continue
  (Default|AttemptProceedtoNextScreen (Variables|Default|GetGame%20Manager))
  (Input|AddMappingContext (PlayerController|LocalPlayerSubsystems|GetEnhancedInputLocalPlayerSubsystem self) "/Game/Input/IMC_Default.IMC_Default" 0 "(bIgnoreAllPressedKeysUntilRelease=True,bForceImmediately=False,bNotifyUserSettings=False)"))

(event Input|EnhancedActionEvents|EnhancedInputActionIA_NavigateHorizontal
  (params (ActionValue :type Float%20%28double-precision%29) (ElapsedSeconds :type Float%20%28double-precision%29) (TriggeredSeconds :type Float%20%28double-precision%29) (InputAction :type Input%20Action%20Object%20Reference :default "/Game/Input/Actions/IA_NavigateHorizontal.IA_NavigateHorizontal"))
  (bind _myplayerindex (Variables|Default|GetMyPlayerIndex))
  ;[1 1 1] Input trigger for player selecting character
  (:Started
    (if (!= _myplayerindex -1)
      (Default|HandleCharacterSelection (Variables|Default|GetGame%20Manager) _myplayerindex ActionValue))))

(event EventBeginPlay
  ;[1 1 1] Mapping context for character select
  (bind _outactors (Actor|GetAllActorsOfClass "/Game/Blueprints/CharacterSelectLogic/CharSelectGameManager.CharSelectGameManager_C"))
  (for _array_element _outactors
    (Variables|Default|SetGame%20Manager _array_element))
  (Utilities|FlowControl|Delay 0.2)
  (CallFunction|SetPlayer))

(fn ConstructionScript)

(fn SetMyPlayerIndex
  (params (Index :type Integer))
  (Variables|Default|SetMyPlayerIndex Index))

(fn SetPlayer
  (bind _self self)
  (bind _returnvalue (PlayerController|LocalPlayerSubsystems|GetEnhancedInputLocalPlayerSubsystem _self))
  (if (Utilities|IsValid _returnvalue)
    (Input|AddMappingContext _returnvalue "/Game/Input/IMC_CharSelect.IMC_CharSelect" 1 "(bIgnoreAllPressedKeysUntilRelease=True,bForceImmediately=False,bNotifyUserSettings=False)")
    (Input|SetInputModeGameandUI _self (Variables|Default|GetJoin%20widget) "DoNotLock" false false)
    (Class|Actor|CreateInputComponent "/Script/EnhancedInput.EnhancedInputComponent")
    (Input|EnableInput _self)))