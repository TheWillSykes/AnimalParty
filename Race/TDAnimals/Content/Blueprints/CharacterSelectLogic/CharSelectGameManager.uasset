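; Manager for the four-player animal character select screen that creates local players and stores player and roster data in the game instance.
; InitializeScreen seeds six animals and four coloured slots, then join attempts claim a free slot by controller ID with an unhighlighted character.
; Selection input cycles the highlight with wraparound and refreshes the widget.
; Proceeding requires one joined player and no duplicate picks before opening AnimalRaceTest, otherwise showing an error.
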(event EventBeginPlay
  (for _index (range 0 3)
    (Class|GameplayStatics|CreatePlayer _index)))

(event Collision|EventActorBeginOverlap
  (params (OtherActor :type Actor%20Object%20Reference)))

(event EventTick
  (params (DeltaSeconds :type Float%20%28single-precision%29)))

(fn ConstructionScript)

(fn HandlePlayerJoinAttempt
  (params (RequestingController :type BP%20Character%20Controller%20Object%20Reference))
  (bind _self self)
  (bind _instance (CallFunction|GetAnimalGameInstance _self))
  (bind _playerdata (Variables|/Game/Blueprints/BP_Game_Instance.BP_Game_Instance_C|GetPlayerData _instance))
  (bind _characterroster (Variables|/Game/Blueprints/BP_Game_Instance.BP_Game_Instance_C|GetCharacterRoster _instance))
  ;[1 1 1] Check if player has already joined, return if true
  (bind _output_get (LocalVariables|SetLocalControlerID (Class|GameplayStatics|GetPlayerControllerID RequestingController)))
  (for _array_element _playerdata
    (if (== (.ControllerID (Utilities|Struct|BreakS_PlayerData _array_element)) _output_get)
      (return)))
  ;[1 1 1] Set player structure data to joined
  (bind (_array_element_2 _array_index) (Utilities|Array|ForEachLoopwithBreak _playerdata :!label _label)
    (:LoopBody
      (if (Utilities|Enum|Equal(Enum) (.JoinStatus (Utilities|Struct|BreakS_PlayerData _array_element_2)) "NewEnumerator0")
        (Utilities|Array|SetArrayElem _playerdata _array_index (Utilities|Struct|MakeS_PlayerData "NewEnumerator1" _output_get (.AssignedColour (Utilities|Struct|BreakS_PlayerData _array_element_2)) -1 false (.ChosenCharacter (Utilities|Struct|BreakS_PlayerData _array_element_2))))
        (Default|SetMyPlayerIndex RequestingController _array_index)
        ;[1 1 1] Find available characters
        (bind _characterindex (CallFunction|FindFirstAvailableCharacter))
        (if (== _characterindex -1)
          (return)
          (else
            ;[1 1 1] Remake player data structure
            (Utilities|Array|SetArrayElem _characterroster _characterindex (Utilities|Struct|MakeS_CharacterData (.CharacterName (Utilities|Struct|BreakS_CharacterData (Utilities|Array|Get(acopy) _characterroster _characterindex))) (.CharacterImage (Utilities|Struct|BreakS_CharacterData (Utilities|Array|Get(acopy) _characterroster _characterindex))) _array_index (.AnimalType (Utilities|Struct|BreakS_CharacterData (Utilities|Array|Get(acopy) _characterroster _characterindex)))))
            (Utilities|Array|SetArrayElem _playerdata _array_index (Utilities|Struct|MakeS_PlayerData (.JoinStatus (Utilities|Struct|BreakS_PlayerData (Utilities|Array|Get(acopy) _playerdata _array_index))) (.ControllerID (Utilities|Struct|BreakS_PlayerData (Utilities|Array|Get(acopy) _playerdata _array_index))) (.AssignedColour (Utilities|Struct|BreakS_PlayerData (Utilities|Array|Get(acopy) _playerdata _array_index))) _characterindex false (.ChosenCharacter (Utilities|Struct|BreakS_PlayerData (Utilities|Array|Get(acopy) _playerdata _array_index)))))
            (Default|UpdateUIVisuals (Variables|Default|GetCharSelectWidget) _array_index)
            (goto _label Break)))))))

(fn FindFirstAvailableCharacter
  ;[1 1 1] Finds empty character slot (-1)
  (bind (_array_element _array_index) (Utilities|Array|ForEachLoopwithBreak (Variables|/Game/Blueprints/BP_Game_Instance.BP_Game_Instance_C|GetCharacterRoster (CallFunction|GetAnimalGameInstance self)))
    (:LoopBody
      (if (== (.HighlightedByPlayerIndex (Utilities|Struct|BreakS_CharacterData _array_element)) -1)
        (return _array_index)))
    (:Completed
      (return -1))))

(fn HandleCharacterSelection
  (params (PlayerIndex :type Integer) (Direction :type Float%20%28double-precision%29))
  (bind _self self)
  (bind _instance (CallFunction|GetAnimalGameInstance _self))
  (bind _playerdata (Variables|/Game/Blueprints/BP_Game_Instance.BP_Game_Instance_C|GetPlayerData _instance))
  (bind _output (Utilities|Array|Get(acopy) _playerdata PlayerIndex))
  (bind _output_2 (Utilities|Array|Get(acopy) _playerdata PlayerIndex))
  (bind (_joinstatus _controllerid _assignedcolour _highlightedcharindex) (Utilities|Struct|BreakS_PlayerData _output))
  (bind (_joinstatus_2 _controllerid_2 _assignedcolour_2) (Utilities|Struct|BreakS_PlayerData _output_2))
  (Development|PrintString (Utilities|String|ToString(Integer) _highlightedcharindex))
  ;[0 0 0] Check if player joined
  (if (Utilities|Enum|Equal(Enum) _joinstatus "NewEnumerator1")
    ;[0 0 0] Clear current highlighted character
    (LocalVariables|SetNumCharacters (Utilities|Array|Length (Variables|/Game/Blueprints/BP_Game_Instance.BP_Game_Instance_C|GetCharacterRoster _instance)))
    (LocalVariables|SetIntDirection (Math|Float|Truncate (Math|Float|Sign(Float) Direction)))
    ;[0 0 0] Update new index, wrap if its exceeding 5
    (bind _output_get (LocalVariables|SetCurrentHighlightIndex%20 (Math|Integer|%(Integer) (+ _highlightedcharindex (LocalVariables|GetIntDirection) (LocalVariables|GetNumCharacters)) (LocalVariables|GetNumCharacters))))
    (switch int _output_get
      (:0
        (Variables|Default|SetChosenChar "NewEnumerator0"))
      (:1
        (Variables|Default|SetChosenChar "NewEnumerator1"))
      (:2
        (Variables|Default|SetChosenChar "NewEnumerator2"))
      (:3
        (Variables|Default|SetChosenChar "NewEnumerator3"))
      (:4
        (Variables|Default|SetChosenChar "NewEnumerator4"))
      (:5
        (Variables|Default|SetChosenChar "NewEnumerator6")))
    ;[0 0 0] Update character and player data, update the UI visuals
    (Utilities|Array|SetArrayElem _playerdata PlayerIndex (Utilities|Struct|MakeS_PlayerData _joinstatus_2 _controllerid_2 _assignedcolour_2 _output_get false (Variables|Default|GetChosenChar)))
    (Default|UpdateUIVisuals (Variables|Default|GetCharSelectWidget) PlayerIndex)
    (return)
    (else
      (return))))

(fn AttemptProceedtoNextScreen
  (bind _self self)
  (bind _usedcharacterindices (LocalVariables|GetUsedCharacterIndices))
  (bind _instance (CallFunction|GetAnimalGameInstance _self))
  (bind _playerdata (Variables|/Game/Blueprints/BP_Game_Instance.BP_Game_Instance_C|GetPlayerData _instance))
  ;[1 1 1] Setup
  (Default|HideErrorMessage (Variables|Default|GetCharSelectWidget))
  ;[1 1 1] Minimum Player Check
  (for _array_element _playerdata
    (if (Utilities|Enum|Equal(Enum) (.JoinStatus (Utilities|Struct|BreakS_PlayerData _array_element)) "NewEnumerator1")
      (LocalVariables|SetNumJoinedPlayers (+ (LocalVariables|GetNumJoinedPlayers) 1))))
  (if (>= (LocalVariables|GetNumJoinedPlayers) 1)
    ;[1 1 1] Duplicate Character Validation
    (for _array_element_2 _playerdata
      (if (Utilities|Enum|Equal(Enum) (.JoinStatus (Utilities|Struct|BreakS_PlayerData _array_element_2)) "NewEnumerator1")
        (if (Utilities|Array|ContainsItem _usedcharacterindices (.HighlightedCharIndex (Utilities|Struct|BreakS_PlayerData _array_element_2)))
          (Default|ShowErrorMessage (Variables|Default|GetCharSelectWidget) "Players cannot select the same character")
          (return)
          (else
            (Utilities|Array|AddUnique _usedcharacterindices (.HighlightedCharIndex (Utilities|Struct|BreakS_PlayerData _array_element_2)))))))
    ;[1 1 1] Check if it needs to be AI
    (for (_array_element_3 _array_index) _playerdata
      (if (Utilities|Enum|Equal(Enum) (.JoinStatus (Utilities|Struct|BreakS_PlayerData _array_element_3)) "NewEnumerator0")
        (Utilities|Array|SetArrayElem _playerdata _array_index (Utilities|Struct|MakeS_PlayerData (.JoinStatus (Utilities|Struct|BreakS_PlayerData _array_element_3)) (.ControllerID (Utilities|Struct|BreakS_PlayerData _array_element_3)) (.AssignedColour (Utilities|Struct|BreakS_PlayerData _array_element_3)) (.HighlightedCharIndex (Utilities|Struct|BreakS_PlayerData _array_element_3)) (.bIsAI (Utilities|Struct|BreakS_PlayerData _array_element_3)) (.ChosenCharacter (Utilities|Struct|BreakS_PlayerData _array_element_3))))))
    (Game|OpenLevel(byObjectReference) "/Game/Maps/LEVELS/RacingLevels/AnimalRaceTest.AnimalRaceTest")
    (else
      (Default|ShowErrorMessage (Variables|Default|GetCharSelectWidget) "At least one player must join")
      (return))))

(fn InitializeScreen
  (params (WidgetRef :type WB%20Char%20Select%20Object%20Reference))
  (bind _self self)
  (bind _instance (CallFunction|GetAnimalGameInstance _self))
  (bind _playerdata (Variables|/Game/Blueprints/BP_Game_Instance.BP_Game_Instance_C|GetPlayerData _instance))
  ;[1 1 1] Makes character data
  (Variables|Default|SetCharSelectWidget WidgetRef)
  (Variables|/Game/Blueprints/BP_Game_Instance.BP_Game_Instance_C|SetCharacterRoster _instance (Utilities|Array|MakeArray (Utilities|Struct|MakeS_CharacterData "Panda" "/Game/Characters/CharacterIconImages/PandaIcon.PandaIcon" -1 "NewEnumerator0") (Utilities|Struct|MakeS_CharacterData "Cheetah" "/Game/Characters/CharacterIconImages/CheetahIcon.CheetahIcon" -1 "NewEnumerator1") (Utilities|Struct|MakeS_CharacterData "Horse" "/Game/Characters/CharacterIconImages/HorseIocn.HorseIocn" -1 "NewEnumerator2") (Utilities|Struct|MakeS_CharacterData "Ostrich" "/Game/Characters/CharacterIconImages/OstrichIcon.OstrichIcon" -1 "NewEnumerator3") (Utilities|Struct|MakeS_CharacterData "Rhino" "/Game/Characters/CharacterIconImages/RhinoIcon.RhinoIcon" -1 "NewEnumerator4") (Utilities|Struct|MakeS_CharacterData "Monkey" "/Game/Characters/CharacterIconImages/MonkeyIcon.MonkeyIcon" -1 "NewEnumerator6")))
  ;[1 1 1] Resets player data
  (Utilities|Array|Clear _playerdata)
  (for _index (range 0 3)
    (Utilities|Array|Add _playerdata (Utilities|Struct|MakeS_PlayerData "NewEnumerator0" -1 (Utilities|Select :Index _index :Option%200 (Class|KismetMathLibrary|LinearColorRed) :Option%201 (Class|KismetMathLibrary|LinearColorGreen) :Option%202 (Class|KismetMathLibrary|LinearColorYellow) :Option%203 (Class|KismetMathLibrary|LinearColorBlue))))
    (Default|UpdateUIVisuals (Variables|Default|GetCharSelectWidget) _index)))