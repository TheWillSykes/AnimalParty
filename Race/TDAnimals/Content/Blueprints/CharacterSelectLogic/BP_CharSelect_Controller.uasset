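; Player controller for the local multiplayer character select screen, turning each player's input into join, character choice and continue requests.
; On BeginPlay it caches the CharSelectGameManager, then applies the character select mapping context and Game-and-UI input mode to up to four local players.
; Enhanced Input events forward to the manager, with MyPlayerIndex (-1 until assigned through SetMyPlayerIndex) gating join and navigation, while continue is ungated.
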(event Custom|StartPlayer
  (params (NewParam :type Boolean)))

(event Input|EnhancedActionEvents|EnhancedInputActionIA_Join
  (params (ActionValue :type Boolean) (ElapsedSeconds :type Float%20%28double-precision%29) (TriggeredSeconds :type Float%20%28double-precision%29) (InputAction :type Input%20Action%20Object%20Reference :default "/Game/Input/Actions/IA_Join.IA_Join"))
  ;[1 1 1] Input trigger for player joining the game
  (:Started
    (if (== (Variables|Default|GetMyPlayerIndex) -1)
      (Default|HandlePlayerJoinAttempt (Variables|Default|GetGame%20Manager) self))))

(event Input|EnhancedActionEvents|EnhancedInputActionIA_NavigateHorizontal
  (params (ActionValue :type Float%20%28double-precision%29) (ElapsedSeconds :type Float%20%28double-precision%29) (TriggeredSeconds :type Float%20%28double-precision%29) (InputAction :type Input%20Action%20Object%20Reference :default "/Game/Input/Actions/IA_NavigateHorizontal.IA_NavigateHorizontal"))
  (bind _myplayerindex (Variables|Default|GetMyPlayerIndex))
  ;[1 1 1] Input trigger for player selecting character
  (:Started
    (if (!= _myplayerindex -1)
      (Default|HandleCharacterSelection (Variables|Default|GetGame%20Manager) _myplayerindex ActionValue))))

(event Input|EnhancedActionEvents|EnhancedInputActionIA_ActivateContinue
  (params (ActionValue :type Boolean) (ElapsedSeconds :type Float%20%28double-precision%29) (TriggeredSeconds :type Float%20%28double-precision%29) (InputAction :type Input%20Action%20Object%20Reference :default "/Game/Input/Actions/IA_ActivateContinue.IA_ActivateContinue"))
  ;[1 1 1] Input trigger for player continue
  (Default|AttemptProceedtoNextScreen (Variables|Default|GetGame%20Manager)))

(event EventBeginPlay
  (Development|PrintString "Hello")
  (bind _outactors (Actor|GetAllActorsOfClass "/Game/Blueprints/CharacterSelectLogic/CharSelectGameManager.CharSelectGameManager_C"))
  (for _array_element _outactors
    (Variables|Default|SetGame%20Manager _array_element)
    ;[1 1 1] Mapping context for character select
    (for _index (range 0 3)
      (if (Utilities|IsValid (PlayerController|LocalPlayerSubsystems|GetEnhancedInputLocalPlayerSubsystem (Game|GetPlayerController _index)))
        (Input|AddMappingContext (PlayerController|LocalPlayerSubsystems|GetEnhancedInputLocalPlayerSubsystem (Game|GetPlayerController _index)) "/Game/Input/IMC_CharSelect.IMC_CharSelect" 0 "(bIgnoreAllPressedKeysUntilRelease=True,bForceImmediately=False,bNotifyUserSettings=False)")
        (Input|SetInputModeGameandUI (Game|GetPlayerController _index) (Variables|Default|GetJoin%20widget) "DoNotLock" false false)))))

(fn ConstructionScript)

(fn SetMyPlayerIndex
  (params (Index :type Integer))
  (Variables|Default|SetMyPlayerIndex Index))