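; Player controller for the race level select screen, letting only the host player pick a level.
; On BeginPlay it caches the RaceLevelSelectGameManager, adds the IMC_CharSelect Enhanced Input mapping and enables input.
; Navigate and continue inputs forward to the manager's level navigation and confirm functions, while go-back opens the game mode select level.
; Every action first checks the controller's ID against the manager's HostControllerID.
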(event Input|EnhancedActionEvents|EnhancedInputActionIA_GoBack
  (params (ActionValue :type Boolean) (ElapsedSeconds :type Float%20%28double-precision%29) (TriggeredSeconds :type Float%20%28double-precision%29) (InputAction :type Input%20Action%20Object%20Reference :default "/Game/Input/Actions/IA_GoBack.IA_GoBack"))
  (:Completed
    (if (== (Variables|/Game/Blueprints/GamemodeSelectLogic/RaceLevelSelect/RaceLevelSelectGameManager.RaceLevelSelectGameManager_C|GetHostControllerID (Variables|Default|GetGame%20Manager)) (Class|GameplayStatics|GetPlayerControllerID self))
      (Game|OpenLevel(byObjectReference) "/Game/Maps/L_GameModeSelect.L_GameModeSelect"))))

(event Input|EnhancedActionEvents|EnhancedInputActionIA_ActivateContinue
  (params (ActionValue :type Boolean) (ElapsedSeconds :type Float%20%28double-precision%29) (TriggeredSeconds :type Float%20%28double-precision%29) (InputAction :type Input%20Action%20Object%20Reference :default "/Game/Input/Actions/IA_ActivateContinue.IA_ActivateContinue"))
  (bind _game_manager (Variables|Default|GetGame%20Manager))
  ;[1 1 1] Input trigger for player continue
  (:Completed
    (if (== (Variables|/Game/Blueprints/GamemodeSelectLogic/RaceLevelSelect/RaceLevelSelectGameManager.RaceLevelSelectGameManager_C|GetHostControllerID _game_manager) (Class|GameplayStatics|GetPlayerControllerID self))
      (Default|ConfirmLevel _game_manager))))

(event Input|EnhancedActionEvents|EnhancedInputActionIA_NavigateHorizontal
  (params (ActionValue :type Float%20%28double-precision%29) (ElapsedSeconds :type Float%20%28double-precision%29) (TriggeredSeconds :type Float%20%28double-precision%29) (InputAction :type Input%20Action%20Object%20Reference :default "/Game/Input/Actions/IA_NavigateHorizontal.IA_NavigateHorizontal"))
  (bind _game_manager (Variables|Default|GetGame%20Manager))
  ;[1 1 1] Input trigger for player selecting character
  (:Started
    (if (== (Variables|/Game/Blueprints/GamemodeSelectLogic/RaceLevelSelect/RaceLevelSelectGameManager.RaceLevelSelectGameManager_C|GetHostControllerID _game_manager) (Class|GameplayStatics|GetPlayerControllerID self))
      (Default|NavigateLevels _game_manager ActionValue))))

(event EventBeginPlay
  (bind _self self)
  (bind _returnvalue (PlayerController|LocalPlayerSubsystems|GetEnhancedInputLocalPlayerSubsystem _self))
  ;[1 1 1] Mapping context for character select
  (bind _outactors (Actor|GetAllActorsOfClass "/Game/Blueprints/GamemodeSelectLogic/RaceLevelSelect/RaceLevelSelectGameManager.RaceLevelSelectGameManager_C"))
  (for _array_element _outactors
    (Variables|Default|SetGame%20Manager _array_element))
  (if (Utilities|IsValid _returnvalue)
    (Input|AddMappingContext _returnvalue "/Game/Input/IMC_CharSelect.IMC_CharSelect" 1 "(bIgnoreAllPressedKeysUntilRelease=True,bForceImmediately=False,bNotifyUserSettings=False)")
    (Class|Actor|CreateInputComponent "/Script/EnhancedInput.EnhancedInputComponent")
    (Input|EnableInput _self)))

(fn ConstructionScript)