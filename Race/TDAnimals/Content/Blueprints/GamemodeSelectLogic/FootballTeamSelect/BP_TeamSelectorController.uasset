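; Player controller for the football team select screen, passing each player's input to the TeamSelectGameManager.
; On BeginPlay it finds its player index by controller ID in the game instance's PlayerData, then after a short delay adds the character select mapping context.
; Horizontal navigation sends selection changes to the manager.
; Only the host, the first non-AI player, can request the next screen or return to game mode select.
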(event Input|EnhancedActionEvents|EnhancedInputActionIA_GoBack
  (params (ActionValue :type Boolean) (ElapsedSeconds :type Float%20%28double-precision%29) (TriggeredSeconds :type Float%20%28double-precision%29) (InputAction :type Input%20Action%20Object%20Reference :default "/Game/Input/Actions/IA_GoBack.IA_GoBack"))
  ;[1 1 1] Go back
  (:Completed
    (if (== (Class|GameplayStatics|GetPlayerControllerID self) (Variables|Default|GetHostControllerID))
      (Game|OpenLevel(byObjectReference) "/Game/Maps/L_GameModeSelect.L_GameModeSelect"))))

(event Input|EnhancedActionEvents|EnhancedInputActionIA_ActivateContinue
  (params (ActionValue :type Boolean) (ElapsedSeconds :type Float%20%28double-precision%29) (TriggeredSeconds :type Float%20%28double-precision%29) (InputAction :type Input%20Action%20Object%20Reference :default "/Game/Input/Actions/IA_ActivateContinue.IA_ActivateContinue"))
  ;[1 1 1] Input trigger for player continue
  (:Completed
    (if (== (Class|GameplayStatics|GetPlayerControllerID self) (Variables|Default|GetHostControllerID))
      (Default|AttemptProceedtoNextScreen (Variables|Default|GetGame%20Manager)))))

(event Input|EnhancedActionEvents|EnhancedInputActionIA_NavigateHorizontal
  (params (ActionValue :type Float%20%28double-precision%29) (ElapsedSeconds :type Float%20%28double-precision%29) (TriggeredSeconds :type Float%20%28double-precision%29) (InputAction :type Input%20Action%20Object%20Reference :default "/Game/Input/Actions/IA_NavigateHorizontal.IA_NavigateHorizontal"))
  ;[1 1 1] Input trigger for player selecting character
  (:Started
    (Default|HandleCharacterSelection (Variables|Default|GetGame%20Manager) (Variables|Default|GetMyPlayerIndex) ActionValue)))

(event EventBeginPlay
  (bind _array_element (Utilities|Array|ForEachLoopwithBreak (Variables|/Game/Blueprints/BP_Game_Instance.BP_Game_Instance_C|GetPlayerData (CallFunction|GetAnimalGameInstance self)) :!label _label)
    (:LoopBody
      (if (== (.ControllerID (Utilities|Struct|BreakS_PlayerData _array_element)) (Class|GameplayStatics|GetPlayerControllerID self))
        ;[1 1 1] Mapping context for character select
        (Variables|Default|SetMyPlayerIndex (.Index (Utilities|Struct|BreakS_PlayerData _array_element)))
        (goto _label Break)))
    (:Completed
      (bind _outactors (Actor|GetAllActorsOfClass "/Game/Blueprints/GamemodeSelectLogic/FootballTeamSelect/TeamSelectGameManager.TeamSelectGameManager_C"))
      (for _array_element_2 _outactors
        (Variables|Default|SetGame%20Manager _array_element_2))
      (Utilities|FlowControl|Delay 0.2)
      (CallFunction|SetPlayer)
      (bind _array_element_3 (Utilities|Array|ForEachLoopwithBreak (Variables|/Game/Blueprints/BP_Game_Instance.BP_Game_Instance_C|GetPlayerData (CallFunction|GetAnimalGameInstance self)) :!label _label_2)
        (:LoopBody
          (if (not (.bIsAI (Utilities|Struct|BreakS_PlayerData _array_element_3)))
            (Variables|Default|SetHostControllerID (.ControllerID (Utilities|Struct|BreakS_PlayerData _array_element_3)))
            (goto _label_2 Break)))
        (:Completed
          (Default|HandleCharacterSelection (Variables|Default|GetGame%20Manager) (Variables|Default|GetMyPlayerIndex) 0.0))))))

(fn ConstructionScript)

(fn SetMyPlayerIndex
  (params (Index :type Integer))
  (Variables|Default|SetMyPlayerIndex Index))

(fn SetPlayer
  (bind _self self)
  (bind _returnvalue (PlayerController|LocalPlayerSubsystems|GetEnhancedInputLocalPlayerSubsystem _self))
  (if (Utilities|IsValid _returnvalue)
    (Input|AddMappingContext _returnvalue "/Game/Input/IMC_CharSelect.IMC_CharSelect" 1 "(bIgnoreAllPressedKeysUntilRelease=True,bForceImmediately=False,bNotifyUserSettings=False)")
    (Input|SetInputModeGameandUI _self (Variables|Default|GetJoin%20widget) "DoNotLock" false false)
    (Class|Actor|CreateInputComponent "/Script/EnhancedInput.EnhancedInputComponent")
    (Input|EnableInput _self)))