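; Player controller for the football game that sets up Enhanced Input and supports player joining and character select.
; On BeginPlay it caches the FootballGameManager and adds the default mapping context.
; SetPlayer adds the character-select context at the same priority, without removing the default, and switches to Game-and-UI input focused on the join widget.
; SetMyPlayerIndex stores the controller's player index.
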(event EventBeginPlay
  (bind _self self)
  (bind _returnvalue (PlayerController|LocalPlayerSubsystems|GetEnhancedInputLocalPlayerSubsystem _self))
  ;[1 1 1] Mapping context for character select
  (bind _outactors (Actor|GetAllActorsOfClass "/Game/Blueprints/FootballLogic/FootballGameManager.FootballGameManager_C"))
  (for _array_element _outactors
    (Variables|Default|SetGame%20Manager _array_element))
  (if (Utilities|IsValid _returnvalue)
    (Input|AddMappingContext _returnvalue "/Game/Input/IMC_Default.IMC_Default" 1 "(bIgnoreAllPressedKeysUntilRelease=True,bForceImmediately=False,bNotifyUserSettings=False)")
    (Class|Actor|CreateInputComponent "/Script/EnhancedInput.EnhancedInputComponent")
    (Input|EnableInput 0)))

(fn ConstructionScript)

(fn SetMyPlayerIndex
  (params (Index :type Integer))
  (Variables|Default|SetMyPlayerIndex Index))

(fn SetPlayer
  (bind _self self)
  (bind _returnvalue (PlayerController|LocalPlayerSubsystems|GetEnhancedInputLocalPlayerSubsystem _self))
  (if (Utilities|IsValid _returnvalue)
    (Input|AddMappingContext _returnvalue "/Game/Input/IMC_CharSelect.IMC_CharSelect" 1 "(bIgnoreAllPressedKeysUntilRelease=True,bForceImmediately=False,bNotifyUserSettings=False)")
    (Input|SetInputModeGameandUI _self (Variables|Default|GetJoin%20widget) "DoNotLock" false false)
    (Class|Actor|CreateInputComponent "/Script/EnhancedInput.EnhancedInputComponent")
    (Input|EnableInput _self)))