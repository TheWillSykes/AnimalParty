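; GoalCounter is a goal trigger actor that tallies scores in an animal football game.
; On BeginPlay it finds and caches the FootballGameManager in the level.
; When an AnimalBall overlaps it, a switch on its Team variable adds one point to that manager's Team1Score or Team2Score.
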(event EventBeginPlay
  (bind _returnvalue (Actor|GetActorOfClass "/Game/Blueprints/FootballLogic/FootballGameManager.FootballGameManager_C"))
  (Variables|Default|SetGamemanager _returnvalue))

(event Collision|EventActorBeginOverlap
  (params (OtherActor :type Actor%20Object%20Reference))
  (bind _gamemanager (Variables|Default|GetGamemanager))
  (Utilities|Casting|CastToAnimalBall OtherActor)
  (switch int (Variables|Default|GetTeam)
    (:0
      (Variables|/Game/Blueprints/FootballLogic/FootballGameManager.FootballGameManager_C|SetTeam1Score _gamemanager (+ (Variables|/Game/Blueprints/FootballLogic/FootballGameManager.FootballGameManager_C|GetTeam1Score _gamemanager) 1)))
    (:1
      (Variables|/Game/Blueprints/FootballLogic/FootballGameManager.FootballGameManager_C|SetTeam2Score _gamemanager (+ (Variables|/Game/Blueprints/FootballLogic/FootballGameManager.FootballGameManager_C|GetTeam2Score _gamemanager) 1)))))

(event EventTick
  (params (DeltaSeconds :type Float%20%28single-precision%29)))

(fn ConstructionScript)